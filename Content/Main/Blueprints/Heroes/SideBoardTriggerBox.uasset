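; SideBoardTriggerBox is a trigger volume that reports overlap state to the RTS player controller.
; On BeginPlay it caches the RTSPlayerControllerBP from player index 0.
; Begin and end overlap write true or false under its own reference into the controller's SideBoardTriggerBoxMap, with no filter on the overlapping actor.
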(event `self.ReceiveBeginPlay`
  (bind _asrtsplayer_controller_bp (cast `/Game/Main/Blueprints/Player/RTSPlayerControllerBP` (`GameplayStatics.GetPlayerController` 0)))
  (set `self.PlayerControllerRef` _asrtsplayer_controller_bp))

(event `self.ReceiveActorEndOverlap`
  (params (OtherActor :type "Actor Object Reference"))
  (`BlueprintMapLibrary.Map_Add` (`/Game/Main/Blueprints/Player/RTSPlayerControllerBP.SideBoardTriggerBoxMap` (`self.PlayerControllerRef`)) self))

(event `self.ReceiveActorBeginOverlap`
  (params (OtherActor :type "Actor Object Reference"))
  (`BlueprintMapLibrary.Map_Add` (`/Game/Main/Blueprints/Player/RTSPlayerControllerBP.SideBoardTriggerBoxMap` (`self.PlayerControllerRef`)) self true))

(fn `UserConstructionScript`)