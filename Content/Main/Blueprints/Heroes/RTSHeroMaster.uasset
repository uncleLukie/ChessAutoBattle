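; RTSHeroMaster is a hero Blueprint that defines stats for the named heroes Aurora, Boris and Countess.
; SetHeroFeatures switches on hero and uses SetHero to bundle name, race, class, tier and combat stats, storing the result for Aurora and Boris.
; The Countess branch repeats Boris's values and stores nothing.
; The construction script is empty, nothing here calls SetHeroFeatures, and dynamic material setup is disabled.
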(fn `SetHero`
  (params (Name :type "/Game/Main/Blueprints/Enums/HeroNamesEnum Enum" :default "NewEnumerator0") (Race :type "/Game/Main/Blueprints/Enums/RacesEnum Enum" :default "NewEnumerator0") (Class :type "/Game/Main/Blueprints/Enums/ClassesEnum Enum" :default "NewEnumerator0") (Tier :type Integer) (AttackSpeed :type "Float (double-precision)") (Damage :type Integer) (Health :type Integer) (Armour :type Integer))
  (returns (Hero :type "/Game/Main/Blueprints/Structures/RTSHeroProfileStruct Structure"))
  (return (make `/Game/Main/Blueprints/Structures/RTSHeroProfileStruct` Name Race Class Tier AttackSpeed Damage Health Armour)))

(fn `SetHeroFeatures`
  (locals (MaterialInstanceLocal :type "MaterialInstanceDynamic Object Reference"))
  (switch `/Game/Main/Blueprints/Enums/HeroNamesEnum` "NewEnumerator0"
    (:`NewEnumerator0`
      (bind _hero (`self.SetHero` "NewEnumerator0" "NewEnumerator0" "NewEnumerator2" 1 1.0 10 100 1))
      (set `self.Aurora` _hero))
    (:`NewEnumerator1`
      (bind _hero_2 (`self.SetHero` "NewEnumerator1" "NewEnumerator2" "NewEnumerator0" 2 1.5 30 100 3))
      (set `self.Boris` _hero_2))
    (:`NewEnumerator2`
      (`self.SetHero` "NewEnumerator1" "NewEnumerator2" "NewEnumerator0" 2 1.5 30 100 3))))

(fn `UserConstructionScript`)