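; Actor Blueprint that defines the stat profiles for the RTS heroes Aurora, Boris, Countess and Crunch.
; MasterHeroProfiles loops up to MaxHeroes, converts each index to the hero name enum and switches on it to fill that hero's variable with hardcoded values.
; SetHero packs name, race, class, tier and combat stats into each profile.
; Its events and construction script are empty, so setup relies on an external call.
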(fn `MasterHeroProfiles`
  (for _index (range (`self.MaxHeroes`))
    (switch `/Game/Main/Blueprints/Enums/HeroNamesEnum` (cast `/Game/Main/Blueprints/Enums/HeroNamesEnum` (`KismetMathLibrary.Conv_IntToByte` _index))
      (:`NewEnumerator0`
        (bind _hero (`self.SetHero` "NewEnumerator0" "NewEnumerator0" "NewEnumerator2" 1 1.0 10 100 1))
        (set `self.Aurora` _hero))
      (:`NewEnumerator1`
        (bind _hero_2 (`self.SetHero` "NewEnumerator1" "NewEnumerator2" "NewEnumerator0" 2 1.5 20 200 3))
        (set `self.Boris` _hero_2))
      (:`NewEnumerator2`
        (bind _hero_3 (`self.SetHero` "NewEnumerator2" "NewEnumerator6" "NewEnumerator3" 3 2.0 15 100 1))
        (set `self.Countess` _hero_3))
      (:`NewEnumerator3`
        (bind _hero_4 (`self.SetHero` "NewEnumerator3" "NewEnumerator4" "NewEnumerator0" 4 2.0 30 400 5))
        (set `self.Crunch` _hero_4))))
  (`KismetSystemLibrary.PrintString` "Hero Profiles Set"))

(fn `SetHero`
  (params (Name :type "/Game/Main/Blueprints/Enums/HeroNamesEnum Enum" :default "NewEnumerator0") (Race :type "/Game/Main/Blueprints/Enums/RacesEnum Enum" :default "NewEnumerator0") (Class :type "/Game/Main/Blueprints/Enums/ClassesEnum Enum" :default "NewEnumerator0") (Tier :type Integer) (AttackSpeed :type "Float (double-precision)") (Damage :type Integer) (Health :type Integer) (Armour :type Integer))
  (returns (Hero :type "/Game/Main/Blueprints/Structures/RTSHeroProfileStruct Structure"))
  (return (make `/Game/Main/Blueprints/Structures/RTSHeroProfileStruct` Name Race Class Tier AttackSpeed Damage Health Armour)))

(fn `UserConstructionScript`)