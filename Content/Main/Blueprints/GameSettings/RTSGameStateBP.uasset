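; RTS game state that runs the in-game clock and calendar, the phased turn cycle and hero stat profiles.
; Tick advances time by game speed and pushes clock and date to the player controller's HUD; speed changes are broadcast.
; A one-second looping timer cycles three phases, allowing player action only in phase 1 and adding base gold each new turn.
; MasterHeroProfiles fills hero structs from an enum loop, but nothing here calls it.
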(event `self.ReceiveBeginPlay`
  (`|ExecutionSequence`
    (:`then_0`
      (`self.ReferenceCasts`))
    (:`then_1`
      ;[1 1 1] Set Default Game Clock and Calendar
      (set `self.GameTime` (+ (`KismetMathLibrary.Conv_IntToDouble` (`self.Hours`)) (/ (`KismetMathLibrary.Conv_IntToDouble` (`self.Minutes`)) 60.0) (/ (`KismetMathLibrary.Conv_IntToDouble` (`self.Hours`)) 3600.0)))
      (set `self.GameDate` (`|MakeArray` (`self.Day`) (`self.Month`) (`self.Year`))))
    (:`then_2`
      ;[1 1 1] Set Default Game Speed
      (set `self.GameSpeed` (`self.DefaultGameSpeed`)))
    (:`then_3`
      (`KismetSystemLibrary.K2_SetTimer` null "DecrementTimer" 1.0 true))))

(event `self.ReceiveTick`
  (params (DeltaSeconds :type "Float (single-precision)"))
  (bind (_gametime _daycount) (`/Game/Main/Blueprints/Library/RTSFunctionLibBP.SetGameTime` DeltaSeconds (`self.GameSpeed`) (`self.GameTime`)))
  ;[1 1 1] Update Game Clock and Calendar
  (set `self.GameTime` _gametime)
  (set `self.DayCounter` _daycount)
  (`self.SetClock`)
  (`self.SetCalendar`))

(event `/Game/Main/Blueprints/Library/RTSGameTimeIFBP.UpdateGameSpeed`
  (params (SpeedMultiplier :type "Float (single-precision)"))
  ;[1 1 1] Update Game Speed
  (bind _output_get (set `self.SpeedMultiplier` SpeedMultiplier))
  (bind _output_get_2 (set `self.GameSpeed` (* _output_get (`self.DefaultGameSpeed`))))
  (`self.GameSpeedControls` _output_get_2))

(fn `CalcGold`
  (locals (BaseIncome :type Integer :default 5))
  (`/Game/Main/Blueprints/Player/RTSPlayerControllerBP.AddGold` (`self.ControllerRef`) (`local.BaseIncome`)))

(fn `CalcWins`)

(fn `DecrementTimer`
  (locals (Phase1Time :type Integer :default 15) (Phase2Time :type Integer :default 10) (Phase3Time :type Integer :default 5))
  (if (== (`self.Timer`) 0)
    (if (== (`self.Phase`) 3)
      (`self.IncTurn`)
      (`self.IncPhase`)
      (set `self.Timer` (`local.Phase1Time`))
      (set `self.CanPlayerAct` true)
      (elif (== (`self.Phase`) 2)
        (`self.IncPhase`)
        (set `self.Timer` (`local.Phase3Time`))
        (set `self.CanPlayerAct` false)
        (else
          (`self.IncPhase`)
          (set `self.Timer` (`local.Phase2Time`))
          (set `self.CanPlayerAct` false)))))
  (bind _output_get (set `self.Timer` (- (`self.Timer`) 1)))
  (`KismetSystemLibrary.PrintString` (`KismetStringLibrary.Conv_IntToString` _output_get)))

(fn `GetGameSpeed`
  (returns (GameSpeed :type "Float (double-precision)"))
  (return (`self.GameSpeed`)))

(fn `IncPhase`
  (if (== (`self.Phase`) 3)
    (set `self.Phase` 1)
    (else
      (set `self.Phase` (+ (`self.Phase`) 1)))))

(fn `IncTurn`
  (bind _result (`/Engine/EditorBlueprintResources/StandardMacros.IncrementInt` (`self.Turn`))
    (:`  `
      (set `self.Turn` _result)
      (`self.CalcGold`))))

(fn `MasterHeroProfiles`
  (locals (MaxHeroes :type Integer))
  (for _index (range (enumcount `/Game/Main/Blueprints/Enums/HeroNamesEnum`))
    (switch `/Game/Main/Blueprints/Enums/HeroNamesEnum` (cast `/Game/Main/Blueprints/Enums/HeroNamesEnum` (`KismetMathLibrary.Conv_IntToByte` _index))
      (:`NewEnumerator0`
        (bind _hero (`self.SetHero` "NewEnumerator0" "NewEnumerator0" "NewEnumerator2" 1 1.0 10 100 1))
        (set `self.Aurora` _hero))
      (:`NewEnumerator1`
        (bind _hero_2 (`self.SetHero` "NewEnumerator1" "NewEnumerator2" "NewEnumerator0" 2 1.5 20 200 3))
        (set `self.Boris` _hero_2))
      (:`NewEnumerator2`
        (bind _hero_3 (`self.SetHero` "NewEnumerator2" "NewEnumerator6" "NewEnumerator3" 3 2.0 15 100 1))
        (set `self.Countess` _hero_3))
      (:`NewEnumerator3`
        (bind _hero_4 (`self.SetHero` "NewEnumerator3" "NewEnumerator4" "NewEnumerator0" 4 2.0 30 400 5))
        (set `self.Crunch` _hero_4))))
  (`KismetSystemLibrary.PrintString` "Hero Profiles Set"))

(fn `SetCalendar`
  (bind _output_get (set `self.Day` (+ (`self.Day`) (`self.DayCounter`))))
  (if (> _output_get (`KismetMathLibrary.DaysInMonth` (`self.Year`) (`self.Month`)))
    (set `self.Day` 1)
    (set `self.Month` (+ (`self.Month`) 1)))
  (if (> (`self.Month`) 12)
    (set `self.Month` 1)
    (set `self.Year` (+ (`self.Year`) 1)))
  (bind _output_get_2 (set `self.GameDate` (`|MakeArray` (`self.Day`) (`self.Month`) (`self.Year`))))
  (message `/Game/Main/Blueprints/Library/RTSGameTimeIFBP.SetGameCalendar` (`/Game/Main/Blueprints/Player/RTSPlayerControllerBP.HUD GameTime Ref` (`self.ControllerRef`)) _output_get_2))

(fn `SetClock`
  (bind (_remainder _returnvalue) (`KismetMathLibrary.FMod` (* (`self.GameTime`) 3600.0) 60.0))
  (bind (_remainder_2 _returnvalue_2) (`KismetMathLibrary.FMod` (`KismetMathLibrary.Conv_IntToDouble` _returnvalue) 60.0))
  (set `self.Seconds` (`KismetMathLibrary.FFloor` _remainder))
  (set `self.Minutes` (`KismetMathLibrary.FFloor` _remainder_2))
  (set `self.Hours` (`KismetMathLibrary.FFloor` (`KismetMathLibrary.FMod` (`KismetMathLibrary.Conv_IntToDouble` _returnvalue_2) 24.0)))
  (bind _output_get (set `self.GameDate` (`|MakeArray` (`self.Seconds`) (`self.Minutes`) (`self.Hours`))))
  (message `/Game/Main/Blueprints/Library/RTSGameTimeIFBP.SetGameClock` (`/Game/Main/Blueprints/Player/RTSPlayerControllerBP.HUD GameTime Ref` (`self.ControllerRef`)) _output_get))

(fn `SetGameCalendar`
  (params (GameDate :type "Array of Integer (by ref)"))
  (returns (Success :type Boolean))
  (return false))

(fn `SetGameClock`
  (params (GameTIme :type "Array of Integer (by ref)"))
  (returns (Success :type Boolean))
  (return false))

(fn `SetHero`
  (params (Name :type "/Game/Main/Blueprints/Enums/HeroNamesEnum Enum" :default "NewEnumerator0") (Race :type "/Game/Main/Blueprints/Enums/RacesEnum Enum" :default "NewEnumerator0") (Class :type "/Game/Main/Blueprints/Enums/ClassesEnum Enum" :default "NewEnumerator0") (Tier :type Integer) (AttackSpeed :type "Float (double-precision)") (Damage :type Integer) (Health :type Integer) (Armour :type Integer))
  (returns (Hero :type "/Game/Main/Blueprints/Structures/RTSHeroProfileStructBP Structure"))
  (return (make `/Game/Main/Blueprints/Structures/RTSHeroProfileStructBP` Name Race Class Tier AttackSpeed Damage Health Armour)))

(fn `SetTimer`
  (if (== (`self.Phase`) 1)
    (set `self.Timer` 15)
    (set `self.CanPlayerAct` true)
    (elif (== (`self.Phase`) 2)
      (set `self.Timer` 10)
      (set `self.CanPlayerAct` false)
      (else
        (set `self.Timer` 5)
        (set `self.CanPlayerAct` false)))))

(fn `UserConstructionScript`)