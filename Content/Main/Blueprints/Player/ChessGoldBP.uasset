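; ChessGoldBP is a player-side Blueprint meant to manage gold, which it stores on the RTS player controller.
; On BeginPlay, a macro casts and caches references to the first player's RTSPlayerControllerBP and the RTSGameStateBP.
; AddGold overwrites the controller's Gold with the passed value instead of adding to it, and RemoveGold is an empty stub.
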(event `self.ReceiveBeginPlay`
  (`|ExecutionSequence`
    (:`then_0`
      (`self.ReferenceMacro`))))

(fn `AddGold`
  (params (Gold :type Integer))
  (set `/Game/Main/Blueprints/Player/RTSPlayerControllerBP.Gold` Gold (`self.PlayerControllerRef`)))

(fn `RemoveGold`)

(fn `UserConstructionScript`)